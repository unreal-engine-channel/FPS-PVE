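; Boss enemy that chases the player, attacks at close range and counts toward the win condition when killed.
; Tick moves it toward the player while DoFollow is set; its Box overlap clears that flag and starts a delayed loop that applies damage and sets the AIAnim attack flag.
; AnyDamage lowers health; at zero it ragdolls, updates the player's kill state and the WinFloor_Actor, then destroys itself after a delay.
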(event OnComponentBeginOverlap(Box)
  (params (OverlappedComponent :type Primitive%20Component%20Object%20Reference) (OtherActor :type Actor%20Object%20Reference) (OtherComp :type Primitive%20Component%20Object%20Reference) (OtherBodyIndex :type Integer) (bFromSweep :type Boolean) (SweepResult :type Hit%20Result%20Structure%20%28by%20ref%29))
  (Variables|Default|SetDoFollow false)
  (Utilities|FlowControl|Delay 1.5 :!label _label)
  (if (Variables|Default|GetDoFollow)
    (Variables|/Game/Blueprints/AI/AIAnim.AIAnim_C|SetDoAttack (Variables|Default|GetAIAnim) false)
    (else
      (Game|Damage|ApplyDamage (Variables|Default|GetPlayer) (Variables|Default|GetAIDamge) 0 0)
      (Variables|/Game/Blueprints/AI/AIAnim.AIAnim_C|SetDoAttack (Variables|Default|GetAIAnim) true)
      (goto _label))))

(event OnComponentEndOverlap(Box)
  (params (OverlappedComponent :type Primitive%20Component%20Object%20Reference) (OtherActor :type Actor%20Object%20Reference) (OtherComp :type Primitive%20Component%20Object%20Reference) (OtherBodyIndex :type Integer))
  (Variables|Default|SetDoFollow true)
  (if (Variables|Default|GetDoFollow) :!label _label
    (Variables|/Game/Blueprints/AI/AIAnim.AIAnim_C|SetDoAttack (Variables|Default|GetAIAnim) false)
    (else
      (Game|Damage|ApplyDamage (Variables|Default|GetPlayer) (Variables|Default|GetAIDamge) 0 0)
      (Variables|/Game/Blueprints/AI/AIAnim.AIAnim_C|SetDoAttack (Variables|Default|GetAIAnim) true)
      (Utilities|FlowControl|Delay 1.5)
      (goto _label))))

(event EventBeginPlay
  (bind _asplayer (Utilities|Casting|CastToPlayer (Game|GetPlayerCharacter 0)))
  (Variables|Default|SetPlayer _asplayer)
  (bind _asaianim (Utilities|Casting|CastToAIAnim (Components|SkeletalMesh|GetAnimInstance (Variables|Character|GetMesh))))
  (Variables|Default|SetAIAnim _asaianim)
  (bind _outactors (Actor|GetAllActorsOfClass "/Game/Blueprints/Actor/WinFloor_Actor.WinFloor_Actor_C"))
  (Variables|Default|SetGameWinBP (Utilities|Array|Get(acopy) _outactors)))

(event Collision|EventActorBeginOverlap
  (params (OtherActor :type Actor%20Object%20Reference)))

(event EventTick
  (params (DeltaSeconds :type Float%20%28single-precision%29))
  (bind _player (Variables|Default|GetPlayer))
  (Utilities|FlowControl|Sequence
    (:then_0
      (if (<= (Variables|Default|GetAIHealth) 0.0)
        (Utilities|FlowControl|DoOnce false
          (:Completed
            (Physics|SetSimulatePhysics (Variables|Character|GetMesh) true)
            (Variables|/Game/Blueprints/Actor/WinFloor_Actor.WinFloor_Actor_C|SetKillEnemy1 (Variables|Default|GetGameWinBP) true)
            (Variables|/Game/Blueprints/Player/Player.Player_C|SetKillEnemyCount _player (+ (Variables|/Game/Blueprints/Player/Player.Player_C|GetKillEnemyCount _player) 1))
            (Variables|/Game/Blueprints/Player/Player.Player_C|SetBossKilled (Variables|Default|GetPlayer) true)
            (Utilities|FlowControl|Delay 3.0)
            (Actor|DestroyActor)))))
    (:then_1
      (if (Variables|Default|GetDoFollow)
        (AI|Navigation|SimpleMovetoActor (AI|GetAIController self) (Variables|Default|GetPlayer))
        (else
          (Components|Movement|StopMovementImmediately (Variables|Character|GetCharacterMovement)))))))

(event Game|Damage|EventAnyDamage
  (params (Damage :type Float%20%28single-precision%29) (DamageType :type Damage%20Type%20Object%20Reference) (InstigatedBy :type Controller%20Object%20Reference) (DamageCauser :type Actor%20Object%20Reference))
  (Variables|Default|SetAIHealth (- (Variables|Default|GetAIHealth) Damage)))

(fn ConstructionScript)