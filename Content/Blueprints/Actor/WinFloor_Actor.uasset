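; WinFloor_Actor is a trigger actor that shows the win screen when its box is overlapped after the player meets a victory condition.
; BeginPlay caches the Player character, whose kill count must equal six or boss-killed flag be set; the overlapping actor is not checked.
; On success it adds the GameWin widget, switches to UI-only input with a visible cursor, then pauses the game after a short delay.
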(event OnComponentBeginOverlap(Box)
  (params (OverlappedComponent :type Primitive%20Component%20Object%20Reference) (OtherActor :type Actor%20Object%20Reference) (OtherComp :type Primitive%20Component%20Object%20Reference) (OtherBodyIndex :type Integer) (bFromSweep :type Boolean) (SweepResult :type Hit%20Result%20Structure%20%28by%20ref%29))
  (bind _returnvalue (Game|GetPlayerController 0))
  (bind _player (Variables|Default|GetPlayer))
  (if (or (== (Variables|/Game/Blueprints/Player/Player.Player_C|GetKillEnemyCount _player) 6) (Variables|/Game/Blueprints/Player/Player.Player_C|GetBossKilled _player))
    (bind _returnvalue_2 (UserInterface|CreateWidget "/Game/Blueprints/UI/GameWin.GameWin_C" _returnvalue))
    (UserInterface|Viewport|AddtoViewport _returnvalue_2 0)
    (Input|SetInputModeUIOnly _returnvalue 0 "DoNotLock")
    (Variables|/Script/Engine.PlayerController|SetbShowMouseCursor _returnvalue true)
    (Utilities|FlowControl|Delay 0.5)
    (Game|SetGamePaused true)))

(event EventBeginPlay
  (bind _asplayer (Utilities|Casting|CastToPlayer (Game|GetPlayerCharacter 0)))
  (Variables|Default|SetPlayer _asplayer))

(event Collision|EventActorBeginOverlap
  (params (OtherActor :type Actor%20Object%20Reference)))

(event EventTick
  (params (DeltaSeconds :type Float%20%28single-precision%29)))

(fn ConstructionScript)