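; BoardTake is an armor pickup actor that refills the player's Armor to full and then destroys itself.
; On BeginPlay it caches the Player character and the first WinFloor_Actor, though the latter is not used afterward.
; Any Box overlap triggers the refill if Armor is below the cap, without checking which actor overlapped; otherwise the pickup stays in place.
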(event OnComponentBeginOverlap(Box)
  (params (OverlappedComponent :type Primitive%20Component%20Object%20Reference) (OtherActor :type Actor%20Object%20Reference) (OtherComp :type Primitive%20Component%20Object%20Reference) (OtherBodyIndex :type Integer) (bFromSweep :type Boolean) (SweepResult :type Hit%20Result%20Structure%20%28by%20ref%29))
  (bind _player (Variables|Default|GetPlayer))
  (if (< (Variables|/Game/Blueprints/Player/Player.Player_C|GetArmor _player) 1e+02)
    (Variables|/Game/Blueprints/Player/Player.Player_C|SetArmor _player 1e+02)
    (Actor|DestroyActor)))

(event EventBeginPlay
  (bind _asplayer (Utilities|Casting|CastToPlayer (Game|GetPlayerCharacter 0)))
  (Variables|Default|SetPlayer _asplayer)
  (bind _outactors (Actor|GetAllActorsOfClass "/Game/Blueprints/Actor/WinFloor_Actor.WinFloor_Actor_C"))
  (Variables|Default|SetGameWinBP (Utilities|Array|Get(acopy) _outactors)))

(event Collision|EventActorBeginOverlap
  (params (OtherActor :type Actor%20Object%20Reference)))

(event EventTick
  (params (DeltaSeconds :type Float%20%28single-precision%29)))

(fn ConstructionScript)