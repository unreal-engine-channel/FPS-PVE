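; Three-stop elevator actor with sliding double doors, driven by number keys while the player's input is enabled.
; BoxUp overlap toggles input and the gates for keys 1 and 2, whose timelines lerp the car up to either upper floor.
; Key 0 closes the doors, reverses the timeline chosen by car height, and reopens after a matching delay.
; BoxOpen overlap and upward arrivals also drive the door timeline.
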(event OnComponentBeginOverlap(BoxOpen)
  (params (OverlappedComponent :type Primitive%20Component%20Object%20Reference) (OtherActor :type Actor%20Object%20Reference) (OtherComp :type Primitive%20Component%20Object%20Reference) (OtherBodyIndex :type Integer) (bFromSweep :type Boolean) (SweepResult :type Hit%20Result%20Structure%20%28by%20ref%29))
  (CallFunction|OpenDoor))

(event OnComponentEndOverlap(BoxOpen)
  (params (OverlappedComponent :type Primitive%20Component%20Object%20Reference) (OtherActor :type Actor%20Object%20Reference) (OtherComp :type Primitive%20Component%20Object%20Reference) (OtherBodyIndex :type Integer))
  (CallFunction|CloseDoor))

(event OnComponentBeginOverlap(BoxUp)
  (params (OverlappedComponent :type Primitive%20Component%20Object%20Reference) (OtherActor :type Actor%20Object%20Reference) (OtherComp :type Primitive%20Component%20Object%20Reference) (OtherBodyIndex :type Integer) (bFromSweep :type Boolean) (SweepResult :type Hit%20Result%20Structure%20%28by%20ref%29))
  (Input|EnableInput (Game|GetPlayerController 0))
  (Utilities|FlowControl|Sequence
    (:then_0
      (Utilities|FlowControl|Gate true) ; enters at Open
    )
    (:then_1
      (Utilities|FlowControl|Gate true) ; enters at Open
    )))

(event OnComponentEndOverlap(BoxUp)
  (params (OverlappedComponent :type Primitive%20Component%20Object%20Reference) (OtherActor :type Actor%20Object%20Reference) (OtherComp :type Primitive%20Component%20Object%20Reference) (OtherBodyIndex :type Integer))
  (Input|DisableInput (Game|GetPlayerController 0))
  (Utilities|FlowControl|Sequence
    (:then_0
      (Utilities|FlowControl|Gate true) ; enters at Close
    )
    (:then_1
      (Utilities|FlowControl|Gate true) ; enters at Close
    )))

(event Custom|BackFromFloor2
  (bind _elevatorlocation (Variables|Default|GetElevatorLocation))
  (bind _alpha (Timeline|Timeline_2 Reverse)
    (:Update
      (Transformation|SetRelativeLocation (Variables|Default|GetElevator) (Math|Vector|MakeVector (.x _elevatorlocation) (.y _elevatorlocation) (Math|Float|Lerp (.z _elevatorlocation) 1e+03 _alpha)) false false))
    (:Finished
      (CallFunction|OpenDoor))))

(event Custom|GoToFloor2
  (bind _elevatorlocation (Variables|Default|GetElevatorLocation))
  (bind _alpha (Timeline|Timeline_2 Play)
    (:Update
      (Transformation|SetRelativeLocation (Variables|Default|GetElevator) (Math|Vector|MakeVector (.x _elevatorlocation) (.y _elevatorlocation) (Math|Float|Lerp (.z _elevatorlocation) 1e+03 _alpha)) false false))
    (:Finished
      (CallFunction|OpenDoor))))

(event Custom|BackFromFloor1
  (bind _elevatorlocation (Variables|Default|GetElevatorLocation))
  (bind _alpha (Timeline|Timeline_1 Reverse)
    (:Update
      (Transformation|SetRelativeLocation (Variables|Default|GetElevator) (Math|Vector|MakeVector (.x _elevatorlocation) (.y _elevatorlocation) (Math|Float|Lerp (.z _elevatorlocation) 5e+02 _alpha)) false false))
    (:Finished
      (CallFunction|OpenDoor))))

(event Custom|GoToFloor1
  (bind _elevatorlocation (Variables|Default|GetElevatorLocation))
  (bind _alpha (Timeline|Timeline_1 Play)
    (:Update
      (Transformation|SetRelativeLocation (Variables|Default|GetElevator) (Math|Vector|MakeVector (.x _elevatorlocation) (.y _elevatorlocation) (Math|Float|Lerp (.z _elevatorlocation) 5e+02 _alpha)) false false))
    (:Finished
      (CallFunction|OpenDoor))))

(event Custom|OpenDoor
  (bind _alpha (Timeline|Timeline_0 Play)
    (:Update
      (Utilities|FlowControl|Sequence
        (:then_0
          (Transformation|SetRelativeLocation (Variables|Default|GetDoorL) (Math|Vector|MakeVector (Math|Float|Lerp 4e+01 1.2e+02 _alpha) -71.333336 0.0) false false))
        (:then_1
          (Transformation|SetRelativeLocation (Variables|Default|GetDoorR) (Math|Vector|MakeVector (Math|Float|Lerp -4e+01 -1.2e+02 _alpha) -71.333336 0.0) false false))))))

(event Custom|CloseDoor
  (bind _alpha (Timeline|Timeline_0 Reverse)
    (:Update
      (Utilities|FlowControl|Sequence
        (:then_0
          (Transformation|SetRelativeLocation (Variables|Default|GetDoorL) (Math|Vector|MakeVector (Math|Float|Lerp 4e+01 1.2e+02 _alpha) -71.333336 0.0) false false))
        (:then_1
          (Transformation|SetRelativeLocation (Variables|Default|GetDoorR) (Math|Vector|MakeVector (Math|Float|Lerp -4e+01 -1.2e+02 _alpha) -71.333336 0.0) false false))))))

(event EventBeginPlay)

(event Collision|EventActorBeginOverlap
  (params (OtherActor :type Actor%20Object%20Reference)))

(event EventTick
  (params (DeltaSeconds :type Float%20%28single-precision%29)))

(event Input|KeyboardEvents|1
  (params (Key :type Key%20Structure))
  (:Pressed
    (Utilities|FlowControl|Gate true
      (:Exit
        (CallFunction|GotoFloor1)))))

(event Input|KeyboardEvents|0
  (params (Key :type Key%20Structure))
  (bind _elevator (Variables|Default|GetElevator))
  (bind _returnvalue (Transformation|GetWorldLocation _elevator))
  (bind _returnvalue_2 (> (.z _returnvalue) 6e+02))
  (:Pressed
    (Utilities|FlowControl|Sequence
      (:then_0
        (if _returnvalue_2
          (CallFunction|BackfromFloor2)
          (else
            (CallFunction|BackfromFloor1))))
      (:then_1
        (if _returnvalue_2
          (Utilities|FlowControl|Delay 1e+01)
          (else
            (Utilities|FlowControl|Delay 5.0)))
        (CallFunction|OpenDoor))
      (:then_2
        (CallFunction|CloseDoor)))))

(event Input|KeyboardEvents|2
  (params (Key :type Key%20Structure))
  (:Pressed
    (Utilities|FlowControl|Gate true
      (:Exit
        (CallFunction|GotoFloor2)))))

(fn ConstructionScript)